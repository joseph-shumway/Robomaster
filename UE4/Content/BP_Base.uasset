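; BP_Base is a team base actor with a main body and three panels, configured entirely in the Construction Script.
; It creates dynamic material instances for the body and a shared one for the panels, setting their TeamBlue parameter when the TeamBlue flag is on.
; When IsOpen is set, it offsets and rotates the panels into a static open pose.
; The event graph holds no active logic.
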(event EventBeginPlay)

(event Collision|EventActorBeginOverlap
  (params (OtherActor :type Actor%20Object%20Reference)))

(event EventTick
  (params (DeltaSeconds :type Float%20%28single-precision%29)))

(fn ConstructionScript
  (bind _basepanel_1 (Variables|Default|GetBasePanel%201))
  (Utilities|FlowControl|Sequence
    (:then_0
      (bind _returnvalue (Rendering|Material|CreateDynamicMaterialInstance "/Game/Materials/MI_Base.MI_Base" "None" :!class /Script/Engine.KismetMaterialLibrary))
      (bind _output_get (Variables|Default|SetBaseMaterial _returnvalue))
      (Rendering|Material|SetMaterial (Variables|Default|GetBase) 0 _output_get)
      (if (Variables|Default|GetTeamBlue)
        (Rendering|Material|SetScalarParameterValue (Variables|Default|GetBaseMaterial) "TeamBlue" 1.0 :!class /Script/Engine.MaterialInstanceDynamic)))
    (:then_1
      (bind _returnvalue_2 (Rendering|Material|CreateDynamicMaterialInstance "/Game/Materials/MI_BasePanel.MI_BasePanel" "None" :!class /Script/Engine.KismetMaterialLibrary))
      (bind _output_get_2 (Variables|Default|SetBasePanelMaterial _returnvalue_2))
      (Rendering|Material|SetMaterial (Variables|Default|GetBasePanel%201) 0 _output_get_2)
      (if (Variables|Default|GetTeamBlue)
        (Rendering|Material|SetScalarParameterValue (Variables|Default|GetBasePanelMaterial) "TeamBlue" 1.0 :!class /Script/Engine.MaterialInstanceDynamic)))
    (:then_2
      (if (Variables|Default|GetIs%20Open)
        (Transformation|AddLocalOffset _basepanel_1 "-15.000000,0.000000,5.000000" false false)
        (Transformation|AddLocalRotation _basepanel_1 "35.000000, 0, 0" false false)))))